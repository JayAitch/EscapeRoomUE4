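; Button_BP is a hittable button that reports to a parent Button_Controller_BP and shows whether the hit was correct.
; When its static mesh is hit, it prints a debug string, casts its attach parent to the controller and passes itself to CheckHit.
; The CorrectHit event swaps the mesh to a pulsing hex tile material, and IncorrectHit restores the base material.
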(event `self.StaticMeshComponent.OnComponentHit`
  (params (HitComponent :type "PrimitiveComponent Object Reference") (OtherActor :type "Actor Object Reference") (OtherComp :type "PrimitiveComponent Object Reference") (NormalImpulse :type "Vector Structure") (Hit :type "HitResult Structure (by ref)"))
  (`KismetSystemLibrary.PrintString` "Hello")
  (bind _asbutton_controller_bp (cast `/Game/Button_Controller_BP` (`self.GetAttachParentActor`)))
  (`/Game/Button_Controller_BP.CheckHit` _asbutton_controller_bp self))

(event `IncorrectHit`
  (`PrimitiveComponent.SetMaterial` (`self.StaticMeshComponent`) 0 "/Game/FirstPerson/Meshes/BaseMaterial.BaseMaterial"))

(event `CorrectHit`
  (`PrimitiveComponent.SetMaterial` (`self.StaticMeshComponent`) 0 "/Game/StarterContent/Materials/M_Tech_Hex_Tile_Pulse.M_Tech_Hex_Tile_Pulse"))

(fn `UserConstructionScript`)