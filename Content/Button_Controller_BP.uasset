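; Button_Controller_BP is a puzzle controller that opens a door once its attached buttons are hit in the correct order.
; CheckHit compares the hit target to the attached actor at the current index, then confirms that Button_BP and advances the index.
; A wrong hit resets the index and calls IncorrectHit on every button.
; Completing the sequence opens the first DoorBP found in the level at BeginPlay, so attachment order defines the solution.
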(event `CheckHit`
  (params (Target :type "Actor Object Reference"))
  (bind _outactors (`self.GetAttachedActors`))
  (bind _output (`|GetArrayItem` _outactors (`self.CorrectHitButton`)))
  (if (== _output Target)
    ;[1 1 1] hit Correct button
    (bind _asbutton_bp (cast `/Game/Button_BP` _output))
    (`/Game/Button_BP.CorrectHit` _asbutton_bp)
    (set `self.CorrectHitButton` (+ (`self.CorrectHitButton`) 1))
    (if (== (`self.CorrectHitButton`) (+ (`KismetArrayLibrary.Array_LastIndex` _outactors) 1))
      (`KismetSystemLibrary.PrintString` "opem")
      (`/Game/DoorBP.OpenDoor` (`|GetArrayItem` (stale `self.ReceiveBeginPlay` _outactors))))
    (else
      ;[1 1 1] Hit incorrect button
      (`KismetSystemLibrary.PrintString` "wrong button")
      (set `self.CorrectHitButton` 0)
      (for _array_element (`self.GetAttachedActors`)
        (bind _asbutton_bp_2 (cast `/Game/Button_BP` _array_element))
        (`/Game/Button_BP.IncorrectHit` _asbutton_bp_2)))))

(event `self.ReceiveBeginPlay`
  ;[1 1 1] hit Correct button
  (bind _outactors (`GameplayStatics.GetAllActorsOfClass` "/Game/DoorBP.DoorBP_C")))

(fn `UserConstructionScript`)